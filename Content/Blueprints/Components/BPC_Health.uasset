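; Health component that tracks an actor's current health, defeated state and a temporary "Thanos Mode" invulnerability.
; Health starts at the maximum, and damage and healing functions clamp it, with damage flagging defeat at zero.
; Thanos Mode sets a flag for a given duration through a retriggerable delay, then fires an expiry event dispatcher.
; CanTakeDamage reports false while defeated or in Thanos Mode, though DecreaseHealth does not check it itself.
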(event Custom|SetThanosMode
  (params (ThanosDuration :type Float%20%28single-precision%29))
  (Variables|Default|SetThanosDuration ThanosDuration)
  (Variables|Default|SetIsThanos true)
  (Development|PrintString "Thanos Mode" true true "(R=0.432597,G=0.080591,B=1.000000,A=1.000000)")
  (Utilities|FlowControl|RetriggerableDelay (Variables|Default|GetThanosDuration))
  (Variables|Default|SetIsThanos false)
  (Default|CallThanosModeExpired))

(event EventBeginPlay
  (Variables|Default|SetCurrentHealth (Variables|Default|GetMaxHealth)))

(event EventTick
  (params (DeltaSeconds :type Float%20%28single-precision%29)))

(fn DecreaseHealth
  (params (IncomingDamage :type Float%20%28double-precision%29))
  (Variables|Default|SetCurrentHealth (Math|Float|Max(Float) (- (Variables|Default|GetCurrentHealth) IncomingDamage) 0.0))
  (Variables|Default|SetIsDefeated (<= (Variables|Default|GetCurrentHealth) 0.0)))

(fn CanTakeDamage
  (return (and (not (Variables|Default|GetIsDefeated)) (not (Variables|Default|GetIsThanos)))))

(fn IncreaseHealth
  (params (IncreaseAmount :type Float%20%28double-precision%29))
  (Variables|Default|SetCurrentHealth (Math|Float|Min(Float) (+ IncreaseAmount (Variables|Default|GetCurrentHealth)) (Variables|Default|GetMaxHealth))))