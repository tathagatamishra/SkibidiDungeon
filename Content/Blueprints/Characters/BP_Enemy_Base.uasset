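; Base enemy character that walks on request, damages the hero when its HitBox overlaps the hero's HurtBox, and reports destruction to its spawner.
; BeginPlay starts a looping sprite-flicker timer and switches hit/hurt collision off around BPCHealth's Thanos mode.
; Hits trigger hit stop and a retriggerable stun that blocks walking.
; Defeat disables the HitBox, then after a delay plays death sound and skull-explosion VFX before destroying the actor.
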(event OnComponentBeginOverlap(HitBox)
  (params (OverlappedComponent :type Primitive%20Component%20Object%20Reference) (OtherActor :type Actor%20Object%20Reference) (OtherComp :type Primitive%20Component%20Object%20Reference) (OtherBodyIndex :type Integer) (bFromSweep :type Boolean) (SweepResult :type Hit%20Result%20Structure%20%28by%20ref%29))
  (bind _asbp_hero (Utilities|Casting|CastToBP_Hero OtherActor))
  (if (== (Variables|/Game/Blueprints/Characters/BP_DungeonChar_Base.BP_DungeonChar_Base_C|GetHurtBox _asbp_hero) OtherComp)
    (Game|Damage|ApplyDamage _asbp_hero (Variables|Default|GetEnemyAttackDamage) 0 self)))

(event Custom|WalkTo
  (params (WorldDirection :type Vector))
  (if (CallFunction|CanWalkto)
    (Pawn|Input|AddMovementInput WorldDirection 1.0 false)
    (elif (CallFunction|OnlyStunned)
      _)))

(event Custom|SetStun
  (Variables|Default|SetIsStunned true)
  (Development|PrintString (Utilities|String|Append (Utilities|GetDisplayName self) "  Stunned") true true "(R=1.000000,G=0.000000,B=0.004758,A=1.000000)")
  (Development|PrintString (Utilities|String|Append "Current health  =  " (Utilities|String|ToString(Float) (Variables|/Game/Blueprints/Components/BPC_Health.BPC_Health_C|GetCurrentHealth (Variables|Default|GetBPC_Health)))) true true "(R=1.000000,G=0.000000,B=0.004758,A=1.000000)")
  (Utilities|FlowControl|RetriggerableDelay (Variables|Default|GetEnemyStunDuration))
  (Variables|Default|SetIsStunned false))

(event Custom|HandleDefeat
  (Development|PrintString "Enemy Eleminited" true true "(R=1.000000,G=0.000000,B=0.000000,A=1.000000)")
  (Collision|SetCollisionEnabled (Variables|Default|GetHitBox) "NoCollision")
  (Utilities|FlowControl|Delay (Variables|Default|GetDespawnDelay))
  (Audio|PlaySound2D (Variables|Default|GetEnemyDieSound) 1.0 1.0 0.0 0 0)
  (Game|SpawnActorfromClass "/Game/Blueprints/VFX/BP_VFX_SkullExplosion.BP_VFX_SkullExplosion_C" (Math|Transform|MakeTransform (Transformation|GetActorLocation) "0, 0, 0" "1.000000,1.000000,1.000000") "AlwaysSpawn" "MultiplyWithRoot" 0 0)
  (Actor|DestroyActor))

(event EventBeginPlay
  (|CallParentFunction)
  (bind _returnvalue (Utilities|Time|SetTimerbyEvent (EventDispatchers|CreateEvent :!event SetSpritVisibility) (Variables|Default|GetSpritFlikerInterval) true))
  (Variables|Default|SetFlikerHandle _returnvalue)
  (Collision|SetCollisionEnabled (Variables|Default|GetHitBox) "NoCollision")
  (Default|SetThanosMode (Variables|Default|GetBPC_Health) 2.0)
  (Collision|SetCollisionEnabled (Variables|Default|GetHitBox) "QueryOnly"))

(event EventDestroyed
  (Default|DeadEnemy (Variables|Default|GetOwningSpawner) self))

(fn ConstructionScript
  (|CallParentFunction))

(fn CheckAttack)

(fn CanWalkto
  (return (and (not (Variables|/Game/Blueprints/Components/BPC_Health.BPC_Health_C|GetIsDefeated (Variables|Default|GetBPC_Health))) (not (Variables|Default|GetIsStunned)))))

(fn OnlyStunned
  (return (and (Variables|Default|GetIsStunned) (not (Variables|/Game/Blueprints/Components/BPC_Health.BPC_Health_C|GetIsDefeated (Variables|Default|GetBPC_Health))))))

(fn HandleHitExtra
  (|CallParentFunction)
  (CallFunction|HitStop)
  (CallFunction|SetStun)
  (if (Variables|/Game/Blueprints/Components/BPC_Health.BPC_Health_C|GetIsDefeated (Variables|Default|GetBPC_Health))
    (CallFunction|HandleDefeat)))