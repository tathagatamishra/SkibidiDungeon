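; Player hero Blueprint for a dungeon game, handling movement, sword and bow attacks, health and the heart HUD.
; CanMove gates input on attack, stun and defeat states, which PaperZD animation override callbacks toggle.
; CheckHit damages enemies overlapping the HitBox, while ShootArrow spawns arrows.
; Taking a hit updates hearts, disables the HurtBox and stuns, then either starts a flicker timer or, on defeat, restarts the level after a delay.
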(event Input|EnhancedActionEvents|EnhancedInputActionIA_Move
  (params (ActionValue :type Vector%202D%20Structure) (ElapsedSeconds :type Float%20%28double-precision%29) (TriggeredSeconds :type Float%20%28double-precision%29) (InputAction :type Input%20Action%20Object%20Reference :default "/Game/Input/Actions/IA_Move.IA_Move"))
  (bind (_x _y) (Math|Vector2D|BreakVector2D ActionValue))
  (if (CallFunction|CanMove)
    (Variables|Default|SetDirectionality ActionValue)
    (Pawn|Input|AddMovementInput "1.000000,0.000000,0.000000" _x false)
    (Pawn|Input|AddMovementInput "0.000000,1.000000,0.000000" _y false)))

(event Input|EnhancedActionEvents|EnhancedInputActionIA_Sword
  (params (ActionValue :type Boolean) (ElapsedSeconds :type Float%20%28double-precision%29) (TriggeredSeconds :type Float%20%28double-precision%29) (InputAction :type Input%20Action%20Object%20Reference :default "/Game/Input/Actions/IA_Sword.IA_Sword"))
  (:Started
    (if (CallFunction|CanMove)
      (|PlayAnimationOverridewithCallbacks (Variables|/Script/PaperZD.PaperZDAnimationComponent|GetAnimInstance (Variables|Default|GetAnimationComponent)) "/Game/Blueprints/Characters/Hero/AnimSequences/Attack.Attack" "DefaultSlot" (Variables|Default|GetSwordAttackSpeed) 0.0
        (:then
          (Variables|Default|SetIsAttacking true))
        (:OnCompleted
          (Variables|Default|SetIsAttacking false :!label _label))
        (:OnCancelled
          (goto _label))))))

(event Input|EnhancedActionEvents|EnhancedInputActionIA_Bow
  (params (ActionValue :type Boolean) (ElapsedSeconds :type Float%20%28double-precision%29) (TriggeredSeconds :type Float%20%28double-precision%29) (InputAction :type Input%20Action%20Object%20Reference :default "/Game/Input/Actions/IA_Bow.IA_Bow"))
  (:Started
    (if (and (CallFunction|CanMove) (Variables|Default|GetCanUseBow))
      (|PlayAnimationOverridewithCallbacks (Variables|/Script/PaperZD.PaperZDAnimationComponent|GetAnimInstance (Variables|Default|GetAnimationComponent)) "/Game/Blueprints/Characters/Hero/AnimSequences/Bow.Bow" "DefaultSlot" (Variables|Default|GetBowAttackSpeed) 0.0
        (:then
          (Variables|Default|SetIsAttacking true))
        (:OnCompleted
          (Variables|Default|SetIsAttacking false :!label _label))
        (:OnCancelled
          (goto _label))))))

(event EventBeginPlay
  (|CallParentFunction)
  (Utilities|FlowControl|Sequence
    (:then_0
      (bind _asplayer_controller (Utilities|Casting|CastToPlayerController (Pawn|GetController)))
      (Input|AddMappingContext (PlayerController|LocalPlayerSubsystems|GetEnhancedInputLocalPlayerSubsystem _asplayer_controller) "/Game/Input/IMC_Dungeon.IMC_Dungeon" 0 "(bIgnoreAllPressedKeysUntilRelease=True,bForceImmediately=False,bNotifyUserSettings=False)"))
    (:then_1
      (bind _returnvalue (UserInterface|CreateWidget "/Game/Widgets/WBP_MainHUD.WBP_MainHUD_C"))
      (bind _output_get (Variables|Default|SetMainHud _returnvalue))
      (UserInterface|Viewport|AddtoViewport _output_get 0)
      (Default|InitHearts (Variables|/Game/Widgets/WBP_MainHUD.WBP_MainHUD_C|GetWBP_HealthBox (Variables|Default|GetMainHud)) (Variables|/Game/Blueprints/Components/BPC_Health.BPC_Health_C|GetMaxHealth (Variables|Default|GetBPC_Health))))
    (:then_2
      (Collision|SetCollisionEnabled (Variables|Default|GetHurtBox) "NoCollision")
      (Default|SetThanosMode (Variables|Default|GetBPC_Health) 2.0)
      (Collision|SetCollisionEnabled (Variables|Default|GetHurtBox) "QueryOnly"))
    (:then_3
      (Transformation|SetWorldLocation (Variables|Default|GetSpringArm) (Transformation|GetActorLocation) false false))))

(event EventHandleHitExtra
  (|CallParentFunction)
  (Default|UpdateCurrentHealth (Variables|/Game/Widgets/WBP_MainHUD.WBP_MainHUD_C|GetWBP_HealthBox (Variables|Default|GetMainHud)) (Variables|/Game/Blueprints/Components/BPC_Health.BPC_Health_C|GetCurrentHealth (Variables|Default|GetBPC_Health)))
  (Default|SetThanosMode (Variables|Default|GetBPC_Health) 2.0)
  (Collision|SetCollisionEnabled (Variables|Default|GetHurtBox) "NoCollision")
  (|PlayAnimationOverridewithCallbacks (Variables|/Script/PaperZD.PaperZDAnimationComponent|GetAnimInstance (Variables|Default|GetAnimationComponent)) (Variables|Default|GetGetHitAnimation) "DefaultSlot" 1.0 0.0
    (:then
      (Variables|Default|SetIsStunned true)
      (if (CallFunction|HeroOnlyStunned)
        (Development|PrintString "Hero Stunned" true true "(R=1.000000,G=0.617915,B=0.000000,A=1.000000)")
        (Development|PrintString (Utilities|String|Append "Hero health =  " (Utilities|String|ToString(Float) (Variables|/Game/Blueprints/Components/BPC_Health.BPC_Health_C|GetCurrentHealth (Variables|Default|GetBPC_Health)))) true true "(R=1.000000,G=0.579404,B=0.000000,A=1.000000)")))
    (:OnCompleted
      (Variables|Default|SetIsStunned false :!label _label)
      (CallFunction|HitStop)
      (if (Variables|/Game/Blueprints/Components/BPC_Health.BPC_Health_C|GetIsDefeated (Variables|Default|GetBPC_Health))
        (Class|PaperZDAnimInstance|JumptoNode (Variables|/Script/PaperZD.PaperZDAnimationComponent|GetAnimInstance (Variables|Default|GetAnimationComponent)) "DefeatJump" "None")
        (Utilities|FlowControl|Delay (Variables|Default|GetRestartDelay))
        (bind _returnvalue (Game|GetCurrentLevelName true))
        (Game|OpenLevel(byName) (Utilities|String|StringToName _returnvalue))
        (else
          (bind _returnvalue_2 (Utilities|Time|SetTimerbyEvent (EventDispatchers|CreateEvent :!event SetSpritVisibility) (Variables|Default|GetSpritFlikerInterval) true))
          (Variables|Default|SetFlikerHandle _returnvalue_2))))
    (:OnCancelled
      (goto _label))))

(fn ConstructionScript
  (|CallParentFunction))

(fn CanMove
  (return (Math|Boolean|ANDBoolean (not (Variables|/Game/Blueprints/Components/BPC_Health.BPC_Health_C|GetIsDefeated (Variables|Default|GetBPC_Health))) (not (Variables|Default|GetIsStunned)) (not (Variables|Default|GetIsAttacking)))))

(fn CheckHit
  (Development|PrintString "Hero Hitting" true true "(R=0.000000,G=1.000000,B=0.009166,A=1.000000)")
  (bind _arrayelement (Utilities|Array|ReverseforEachLoop (Collision|GetOverlappingActors (Variables|Default|GetHitBox) "/Game/Blueprints/Characters/BP_Enemy_Base.BP_Enemy_Base_C" :!class /Script/Engine.PrimitiveComponent))
    (:LoopBody
      (bind _returnvalue (Game|Damage|ApplyDamage _arrayelement (Variables|Default|GetSwordDamage) 0 self))
      (Development|PrintString (Utilities|String|Append "Sword Damage =   " (Utilities|String|ToString(Float) _returnvalue)) true true "(R=0.000000,G=1.000000,B=0.009166,A=1.000000)"))))

(fn HeroOnlyStunned
  (return (and (not (Variables|/Game/Blueprints/Components/BPC_Health.BPC_Health_C|GetIsDefeated (Variables|Default|GetBPC_Health))) (Variables|Default|GetIsStunned))))

(fn ShootArrow
  (bind _arrowposition (Variables|Default|GetArrowPosition))
  (bind _returnvalue (Transformation|GetWorldTransform _arrowposition))
  (Game|SpawnActorfromClass "/Game/Blueprints/Projectiles/BP_Arrow.BP_Arrow_C" (Math|Transform|MakeTransform (.location _returnvalue) (.rotation _returnvalue) "1.000000,1.000000,1.000000") "AlwaysSpawn" "MultiplyWithRoot" self 0))

(fn GetHeal
  (params (IncreaseAmount :type Float%20%28double-precision%29))
  (Default|IncreaseHealth (Variables|Default|GetBPC_Health) IncreaseAmount)
  (Default|UpdateCurrentHealth (Variables|/Game/Widgets/WBP_MainHUD.WBP_MainHUD_C|GetWBP_HealthBox (Variables|Default|GetMainHud)) (Variables|/Game/Blueprints/Components/BPC_Health.BPC_Health_C|GetCurrentHealth (Variables|Default|GetBPC_Health))))