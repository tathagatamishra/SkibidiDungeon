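; Base dungeon character Blueprint that provides shared hit reactions for sprite-based combat.
; Damage allowed by BPCHealth lowers health, plays a sound, flashes the sprite red and drives timeline knockback away from the causer.
; It then calls the empty HandleHitExtra hook and freezes the attacking dungeon character briefly through CustomTimeDilation.
; When BPCHealth's Thanos mode expires, it stops the flicker timer, shows the sprite and sets HurtBox to query-only.
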(event Custom|OnThanosModeExpired
  (Development|PrintString "Thanos mode ended" true true "(R=0.300510,G=0.042991,B=1.000000,A=1.000000)")
  (Utilities|Time|ClearandInvalidateTimerbyHandle (Variables|Default|GetFlikerHandle))
  (Rendering|SetVisibility (Variables|Default|GetSprite) true false)
  (Collision|SetCollisionEnabled (Variables|Default|GetHurtBox) "QueryOnly"))

(event Custom|FlashSprite
  (Sprite|SetSpriteColor (Variables|Default|GetSprite) "(R=1.000000,G=0.046875,B=0.046875,A=1.000000)")
  (Utilities|FlowControl|RetriggerableDelay (Variables|Default|GetFlashDuration))
  (Sprite|SetSpriteColor (Variables|Default|GetSprite) "(R=1.000000,G=1.000000,B=1.000000,A=1.000000)"))

(event Custom|HitStop
  (Variables|Default|SetCustomTimeDilation 0.0)
  (Utilities|FlowControl|RetriggerableDelay (Variables|Default|GetHitStopDuration))
  (Variables|Default|SetCustomTimeDilation 1.0))

(event Custom|GetKnockBack
  (params (Attacker :type Actor%20Object%20Reference))
  (Variables|Default|SetKnockBackDirection (Math|Vector|GetForwardVector (Math|Rotator|FindLookatRotation (Transformation|GetActorLocation Attacker) (Transformation|GetActorLocation))))
  (Components|Timeline|SetPlayRate (Variables|Default|GetKnockBackMovement) (Variables|Default|GetKnockBackRate))
  (Timeline|KnockBackMovement PlayFromStart
    (:Update
      (Variables|/Script/Engine.MovementComponent|SetVelocity (Variables|Character|GetCharacterMovement) (* (Variables|Default|GetKnockBackDirection) (Variables|Default|GetKnockBackStrength) (Utilities|Time|GetWorldDeltaSeconds))))))

(event EventBeginPlay
  (EventDispatchers|BindEventtoThanosModeExpired (Variables|Default|GetBPC_Health) (delegate Custom|OnThanosModeExpired)))

(event Game|Damage|EventAnyDamage
  (params (Damage :type Float%20%28single-precision%29) (DamageType :type Damage%20Type%20Object%20Reference) (InstigatedBy :type Controller%20Object%20Reference) (DamageCauser :type Actor%20Object%20Reference))
  (if (Default|CanTakeDamage (Variables|Default|GetBPC_Health))
    (Default|DecreaseHealth (Variables|Default|GetBPC_Health) Damage)
    (Audio|PlaySound2D (Variables|Default|GetHitSound) 1.0 1.0 0.0 0 0)
    (CallFunction|FlashSprite)
    (CallFunction|GetKnockBack DamageCauser)
    (CallFunction|HandleHitExtra)
    (bind _asbp_dungeon_char_base (Utilities|Casting|CastToBP_DungeonChar_Base DamageCauser))
    (CallFunction|HitStop _asbp_dungeon_char_base)))

(fn ConstructionScript)

(fn HandleHitExtra)

(fn SetSpritVisibility
  (Rendering|SetVisibility (Variables|Default|GetSprite) (not (Variables|/Script/Engine.SceneComponent|GetbVisible (Variables|Default|GetSprite))) false))