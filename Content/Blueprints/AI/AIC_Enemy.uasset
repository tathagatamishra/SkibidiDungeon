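; AIC_Enemy is an AI controller that makes a possessed BP_Enemy_Base pawn chase the player.
; It takes player pawn 0 as its target at BeginPlay and stores the cast pawn on possession.
; Each Tick, while the target is valid and farther than StopDistance, it passes the look-at direction toward the player to the pawn's WalkTo, steering straight without pathfinding.
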(event EventBeginPlay
  (Variables|Default|SetTargetPlayer (Game|Player|GetPlayerPawn 0)))

(event EventTick
  (params (DeltaSeconds :type Float%20%28single-precision%29))
  (Utilities|IsValid (Variables|Default|GetTargetPlayer)
    (:Is%20Valid
      (bind _returnvalue (CallFunction|GetTargetDistance))
      (if (> _returnvalue (Variables|Default|GetStopDistance))
        (Default|Walkto (Variables|Default|GetPossessed%20Pawn) (Math|Vector|GetForwardVector (Math|Rotator|FindLookatRotation (Transformation|GetActorLocation (Variables|Default|GetPossessed%20Pawn)) (Transformation|GetActorLocation (Variables|Default|GetTargetPlayer)))))))))

(event EventPossess
  (params (PossessedPawn :type Pawn%20Object%20Reference))
  (bind _asbp_enemy_base (Utilities|Casting|CastToBP_Enemy_Base PossessedPawn))
  (Variables|Default|SetPossessed%20Pawn _asbp_enemy_base))

(fn ConstructionScript)

(fn GetTargetDistance
  (return (Math|Vector|Distance(Vector) (Transformation|GetActorLocation (Variables|Default|GetTargetPlayer)) (Transformation|GetActorLocation (Variables|Default|GetPossessed%20Pawn)))))